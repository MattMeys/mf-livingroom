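; Floor tile for a runner game that extends the track and adds multiplier-scaled score when the runner overlaps its box.
; Unless it is the first tile, construction spawns an obstacle at a random Y offset, plus a nitro when the score is divisible by 20.
; Points too close to the player are sunk below the floor for obstacles or skipped for nitros.
; GetAttachPoint exposes the arrow transform.
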(event OnComponentBeginOverlap(Box)
  (params (OverlappedComponent :type Primitive%20Component%20Object%20Reference) (OtherActor :type Actor%20Object%20Reference) (OtherComp :type Primitive%20Component%20Object%20Reference) (OtherBodyIndex :type Integer) (bFromSweep :type Boolean) (SweepResult :type Hit%20Result%20Structure%20%28by%20ref%29))
  ;[1 1 1] extend floor
  (Utilities|Casting|CastToBP_RunnerCharacter OtherActor)
  (bind _asbp_runner_game_mode (Utilities|Casting|CastToBP_RunnerGameMode (Game|GetGameMode)))
  (Default|ExtendFloor _asbp_runner_game_mode)
  ;[1 1 1] Set Current Score
  (bind _asbp_runner_game_mode_2 (Utilities|Casting|CastToBP_RunnerGameMode (Game|GetGameMode)))
  (Variables|/Game/BP_RunnerGameMode.BP_RunnerGameMode_C|SetCurrentPoints _asbp_runner_game_mode_2 (+ (* (Variables|/Game/BP_RunnerGameMode.BP_RunnerGameMode_C|GetPointsMulti _asbp_runner_game_mode_2) 1) (Variables|/Game/BP_RunnerGameMode.BP_RunnerGameMode_C|GetCurrentPoints _asbp_runner_game_mode_2))))

(event EventBeginPlay)

(event Collision|EventActorBeginOverlap
  (params (OtherActor :type Actor%20Object%20Reference)))

(event EventTick
  (params (DeltaSeconds :type Float%20%28single-precision%29)))

(fn ConstructionScript
  (if (not (Variables|Default|GetisFirst))
    (CallFunction|SetupSpawnPoints)
    (CallFunction|SpawnObstacles)
    (CallFunction|NitroSpawnPoints)
    (CallFunction|SpawnNitros)))

(fn GetAttachPoint
  (return (Transformation|GetWorldTransform (Variables|Default|GetArrow))))

(fn SetupSpawnPoints
  (bind _returnvalue (AddComponent|AddArrowComponent false (Math|Transform|MakeTransform (Math|Vector|MakeVector 0.0 (Math|Random|RandomFloatinRange -7e+02 7e+02) 1.0))))
  ;[1 1 1] block if too close to Player
  (bind _returnvalue_2 (Actor|GetActorOfClass "/Game/BP_RunnerCharacter.BP_RunnerCharacter_C"))
  (if (< (Math|Vector|Distance(Vector) (.Location (Math|Transform|BreakTransform (Transformation|GetWorldTransform _returnvalue))) (Transformation|GetWorldLocation (Variables|/Script/Engine.Character|GetCapsuleComponent _returnvalue_2))) 7e+02)
    (Utilities|Array|Add (Variables|Default|GetSpawnPoints) (Math|Conversions|ToTransform(Vector) (Math|Vector|MakeVector 0.0 0.0 -1e+03)))
    (else
      (Utilities|Array|Add (Variables|Default|GetSpawnPoints) (Transformation|GetWorldTransform _returnvalue)))))

(fn SpawnObstacles
  (bind _output_get (LocalVariables|SetRandsomSpawnPoints (Variables|Default|GetSpawnPoints)))
  (Utilities|Array|Shuffle _output_get)
  (for _index (range 0 0)
    (switch int (Math|Random|RandomIntegerinRange 0 1)
      (:0
        (AddComponent|AddChildActorComponent false (Math|Transform|MakeRelativeTransform (Utilities|Array|Get(acopy) (LocalVariables|GetRandsomSpawnPoints) _index) (Transformation|GetActorTransform))))
      (:1
        (AddComponent|AddChildActorComponent false (Math|Transform|MakeRelativeTransform (Utilities|Array|Get(acopy) (LocalVariables|GetRandsomSpawnPoints) _index) (Transformation|GetActorTransform)))))))

(fn NitroSpawnPoints
  ;[1 1 1] only every 10th floor
  (bind _asbp_runner_game_mode (Utilities|Casting|CastToBP_RunnerGameMode (Game|GetGameMode)))
  (if (== (Math|Integer|%(Integer) (Variables|/Game/BP_RunnerGameMode.BP_RunnerGameMode_C|GetCurrentPoints _asbp_runner_game_mode) 20) 0)
    (bind _returnvalue (AddComponent|AddArrowComponent false (Math|Transform|MakeTransform (Math|Vector|MakeVector 0.0 (Math|Random|RandomFloatinRange -6e+02 6e+02) 1.0))))
    (Components|Arrow|SetArrowColor(LinearColor) _returnvalue "(R=0.000000,G=0.120050,B=1.000000,A=1.000000)")
    ;[1 1 1] block if too close to Player
    (bind _returnvalue_2 (Actor|GetActorOfClass "/Game/BP_RunnerCharacter.BP_RunnerCharacter_C"))
    (if (not (< (Math|Vector|Distance(Vector) (.Location (Math|Transform|BreakTransform (Transformation|GetWorldTransform _returnvalue))) (Transformation|GetWorldLocation (Variables|/Script/Engine.Character|GetCapsuleComponent _returnvalue_2))) 7e+02))
      (Utilities|Array|Add (Variables|Default|GetNitroSpawnPoints) (Transformation|GetWorldTransform _returnvalue)))))

(fn SpawnNitros
  (bind _nitrospawnpoints (Variables|Default|GetNitroSpawnPoints))
  (if (!= (Utilities|Array|Length _nitrospawnpoints) 0)
    (bind _output_get (LocalVariables|SetRandsomSpawnPoints _nitrospawnpoints))
    (Utilities|Array|Shuffle _output_get)
    (for _index (range 0 0)
      (AddComponent|AddChildActorComponent false (Math|Transform|MakeRelativeTransform (Utilities|Array|Get(acopy) (LocalVariables|GetRandsomSpawnPoints) _index) (Transformation|GetActorTransform))))))