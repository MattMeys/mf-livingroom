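; BP_Hoverboard is a hoverboard actor that can spin in kickflip tricks.
; Kickflip activates its RotatingMovement component with a rotation rate picked at random from the KickRotations array, or deactivates it when told to stop.
; When that component deactivates, an event handler snaps the actor's relative rotation back to zero.
; The file contains no hover or riding logic, and Tick is unused.
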(event OnComponentDeactivated(RotatingMovement)
  (params (Component :type Actor%20Component%20Object%20Reference))
  (Transformation|SetActorRelativeRotation "0, 0, 0"))

(event EventBeginPlay)

(event Collision|EventActorBeginOverlap
  (params (OtherActor :type Actor%20Object%20Reference)))

(event EventTick
  (params (DeltaSeconds :type Float%20%28single-precision%29)))

(fn ConstructionScript)

(fn Kickflip
  (params (Start :type Boolean))
  (bind _rotatingmovement (Variables|Default|GetRotatingMovement))
  (if Start
    (Components|Activation|Activate _rotatingmovement false)
    (bind _result (Math|Integer|DecrementInt (Utilities|Array|Length (Variables|Default|GetKickRotations)))
      (:%20%20
        (Variables|/Script/Engine.RotatingMovementComponent|SetRotationRate _rotatingmovement (Utilities|Array|Get(acopy) (Variables|Default|GetKickRotations) (Math|Random|RandomIntegerinRange 0 _result)))))
    (else
      (Components|Activation|Deactivate _rotatingmovement))))