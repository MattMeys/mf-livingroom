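; BP_Senemy is an enemy actor that turns to face the player and slides sideways to match the player's Y position.
; Each Tick it interpolates its yaw toward a look-at rotation on the first player pawn.
; It then closes the Y gap by a delta-time-scaled fraction, keeping X and Z fixed and moving without sweep.
; An FInterpTo alternative for this smoothing is left unconnected.
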(event EventBeginPlay)

(event Collision|EventActorBeginOverlap
  (params (OtherActor :type Actor%20Object%20Reference)))

(event EventTick
  (params (DeltaSeconds :type Float%20%28single-precision%29))
  (bind _returnvalue (Transformation|GetActorLocation))
  (bind _returnvalue_2 (Game|Player|GetPlayerPawn 0))
  (bind _returnvalue_3 (Transformation|GetActorLocation _returnvalue_2))
  (Variables|Default|SetDelta%20Seconds DeltaSeconds)
  ;[1 1 1] look at player
  (Variables|Default|SetPlayer _returnvalue_2)
  (Variables|Default|SetPlayerY (.Y (Math|Vector|BreakVector _returnvalue_3)))
  (Transformation|SetActorRotation (Math|Rotator|MakeRotator 0.0 0.0 (.yaw (Math|Interpolation|RInterpTo (Transformation|GetActorRotation) (Math|Rotator|FindLookatRotation (Transformation|GetActorLocation) _returnvalue_3) (Utilities|Time|GetWorldDeltaSeconds) 15.0))))
  (bind _output_get (Variables|Default|SetSenemyY (.y _returnvalue)))
  (if (> (- (Variables|Default|GetSenemyY) (Variables|Default|GetPlayerY)) 0.0)
    (Variables|Default|SetReturnY (- (Variables|Default|GetSenemyY) (* (Variables|Default|GetDelta%20Seconds) 5.0 (Math|Float|Absolute(Float) (- (Variables|Default|GetSenemyY) (Variables|Default|GetPlayerY))))))
    (else
      (Variables|Default|SetReturnY (+ (Variables|Default|GetSenemyY) (* (Variables|Default|GetDelta%20Seconds) 5.0 (Math|Float|Absolute(Float) (- (Variables|Default|GetSenemyY) (Variables|Default|GetPlayerY))))))))
  (Transformation|SetActorLocation (Math|Vector|MakeVector (.x _returnvalue) (Variables|Default|GetReturnY) (.z _returnvalue)) false false))

(fn ConstructionScript)