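; BP_HeadSlice is a runner obstacle that kills the player on contact.
; On BeginPlay, a coin flip decides whether it keeps its placement or is set to a 180-degree rotation and raised by a small random height, adding layout variety.
; Overlapping a BP_RunnerCharacter calls that character's Death, then pauses the game after a short delay.
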(event EventBeginPlay
  (bind _returnvalue (Transformation|GetActorLocation))
  (|CallParentFunction)
  (if (Math|Random|RandomBool)
    (Transformation|SetActorRotation "0.000000,180.000000,0.000000")
    (Transformation|SetActorLocation (Math|Vector|MakeVector (.x _returnvalue) (.y _returnvalue) (+ (.z _returnvalue) (Math|Random|RandomFloatinRange 0.0 7e+01))) false false)))

(event EventTick
  (params (DeltaSeconds :type Float%20%28single-precision%29))
  (|CallParentFunction DeltaSeconds) ; This node is disabled and will not be called.\nDrag off pins to build functionality.
)

(event Collision|EventActorBeginOverlap
  (params (OtherActor :type Actor%20Object%20Reference))
  (bind _asbp_runner_character (Utilities|Casting|CastToBP_RunnerCharacter OtherActor))
  (Default|Death _asbp_runner_character)
  (Utilities|FlowControl|Delay 2.0)
  (Game|SetGamePaused true))

(fn ConstructionScript
  (|CallParentFunction))